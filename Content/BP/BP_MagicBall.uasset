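; BP_MagicBall is a magic fireball projectile that detaches and launches when ShootBall sets its velocity.
; On overlap, it searches all BP_EnemyAI actors, applying point damage to those overlapping BP_CombatCharacter's MagicBall reference.
; Any overlap calls DestroyBall, which spawns an explosion, sets lifespan to zero (clearing the timer) and deactivates the Niagara effect.
; Discharge instead deactivates the effect and sets a short lifespan.
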(event Custom|ShootBall
  (params (Direction :type Vector) (Speed :type Float%20%28double-precision%29))
  (Transformation|DetachFromActor "KeepWorld" "KeepWorld" "KeepWorld")
  (Variables|/Script/Engine.MovementComponent|SetVelocity (Variables|Default|GetProjectileMovement) (* Direction Speed)))

(event Custom|Destroy%20Ball
  (Game|SpawnActorfromClass "/Game/FX/P_Explosion.P_Explosion_C" (Transformation|GetActorTransform) "AlwaysSpawn" 0 0)
  (Actor|SetLifeSpan 0.0)
  (Components|Activation|Deactivate (Variables|Default|GetNS_FireBall)))

(event Custom|Discharge
  (Components|Activation|Deactivate (Variables|Default|GetNS_FireBall))
  (Actor|SetLifeSpan 2.0))

(event EventBeginPlay)

(event Collision|EventActorBeginOverlap
  (params (OtherActor :type Actor%20Object%20Reference))
  (bind _returnvalue (Actor|GetActorOfClass "/Game/FlexibleCombatSystem/Blueprints/BP_CombatCharacter.BP_CombatCharacter_C"))
  (bind _outactors (Actor|GetAllActorsOfClass "/Game/FlexibleCombatSystem/Blueprints/AI/BP_EnemyAI.BP_EnemyAI_C"))
  (for _array_element _outactors
    (if (Collision|IsOverlappingActor _array_element (Variables|/Game/FlexibleCombatSystem/Blueprints/BP_CombatCharacter.BP_CombatCharacter_C|GetMagic%20Ball _returnvalue) :!class /Script/Engine.Actor)
      (Game|Damage|ApplyPointDamage _array_element 25.0 (Math|Vector|MakeVector 0.0 0.0 0.0) (Collision|MakeHitResult false false 0.0 0.0 "0, 0, 0" "0, 0, 0" "0,0,1" "0,0,1" 0 0))
      (CallFunction|DestroyBall)))
  (CallFunction|DestroyBall))

(fn ConstructionScript)