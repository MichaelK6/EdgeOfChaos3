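; Implosion spell component that swells its owner's "Sphere"-tagged mesh, then collapses it while sucking in nearby physics objects.
; When its per-frame Timer hits zero, the hidden sphere appears with an attached sound.
; Tick changes the sphere's volume linearly via cube-root scaling, growing until frame 120, then shrinking faster.
; During collapse, simulating StaticMeshActors in range get an inward force that fades with distance, and the owner is destroyed at zero scale.
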(event EventBeginPlay
  (Rendering|SetVisibility (Utilities|Array|Get(acopy) (Actor|GetComponentsbyTag (Components|GetOwner) "/Script/Engine.StaticMeshComponent" "Sphere")) false true)
  (Class|GameplayStatics|PrimeSound "/Game/DavidsStuff/Spells/SFX/Implode_Cue.Implode_Cue"))

(event EventTick
  (params (DeltaSeconds :type Float%20%28single-precision%29))
  (bind _returnvalue (Components|GetOwner))
  (bind _returnvalue_2 (Math|Trig|GetPI))
  (bind _timer (Variables|Default|GetTimer))
  (bind _returnvalue_3 (Actor|GetComponentsbyTag _returnvalue "/Script/Engine.StaticMeshComponent" "Sphere"))
  (bind _returnvalue_4 (Actor|GetComponentbyClass _returnvalue "/Script/Engine.StaticMeshComponent"))
  (bind _returnvalue_5 (< _timer 120))
  (bind _output (Utilities|Array|Get(acopy) _returnvalue_3))
  (bind _returnvalue_6 (select _returnvalue_5 1e+01 -1e+02))
  (bind _relativescale3d (Variables|/Script/Engine.SceneComponent|GetRelativeScale3D _returnvalue_4))
  (bind _returnvalue_7 (Transformation|GetWorldLocation _output))
  (bind _returnvalue_8 (* _returnvalue_6 0.75))
  (bind _relativescale3d_2 (Variables|/Script/Engine.SceneComponent|GetRelativeScale3D _output))
  (bind _returnvalue_9 (/ _returnvalue_8 _returnvalue_2))
  (bind _returnvalue_10 (* _relativescale3d_2 _relativescale3d))
  (bind (_x _y _z) (Math|Vector|BreakVector _returnvalue_10))
  (bind _returnvalue_11 (* _x _y _z))
  (bind _returnvalue_12 (Math|Float|Power _returnvalue_11 0.333333))
  (bind _returnvalue_13 (+ _returnvalue_9 _returnvalue_11))
  (bind _returnvalue_14 (Math|Float|Max(Float) _returnvalue_13 0.0))
  (bind _returnvalue_15 (/ _returnvalue_10 _returnvalue_12))
  (bind _returnvalue_16 (Math|Float|Power _returnvalue_14 0.333333))
  (bind _returnvalue_17 (* _returnvalue_16 _returnvalue_15))
  (Math|Integer|IncrementInt _timer
    (:%20%20
      (if (== _timer 0)
        (Rendering|SetVisibility _output true true)
        (Audio|SpawnSoundAttached "/Game/DavidsStuff/Spells/SFX/Implode_Cue.Implode_Cue" _output "None" "0, 0, 0" "0, 0, 0" "SnapToTargetIncludingScale" false 1.0 1.0 0.0 0 0))
      (Transformation|SetRelativeScale3D _output (/ _returnvalue_17 _relativescale3d))
      (Utilities|FlowControl|Sequence
        (:then_0
          (if (not _returnvalue_5)
            (bind _outactors (Actor|GetAllActorsOfClass "/Script/Engine.StaticMeshActor"))
            (for _array_element _outactors
              (bind _asstatic_mesh_actor (Utilities|Casting|CastToStaticMeshActor _array_element))
              (if (<= (Math|Vector|Distance(Vector) _returnvalue_7 (Transformation|GetWorldLocation (Variables|/Script/Engine.Actor|GetRootComponent _asstatic_mesh_actor))) 1e+04)
                (if (Physics|IsSimulatingPhysics (Variables|/Script/Engine.StaticMeshActor|GetStaticMeshComponent _asstatic_mesh_actor) "None")
                  (CallFunction|AddForceTowards (Variables|/Script/Engine.StaticMeshActor|GetStaticMeshComponent _asstatic_mesh_actor) _returnvalue_7 (* (/ (- 1e+04 (Math|Vector|Distance(Vector) _returnvalue_7 (Transformation|GetWorldLocation (Variables|/Script/Engine.Actor|GetRootComponent _asstatic_mesh_actor)))) 1e+04) 1e+06) false))))))
        (:then_1
          (if (Utilities|Operators|EqualEqual :A _returnvalue_17 :ErrorTolerance 0.0)
            (Actor|DestroyActor _returnvalue)))))))

(fn AddForceTowards
  (params (Target :type Primitive%20Component%20Object%20Reference) (Destination :type Vector) (Strength :type Float%20%28double-precision%29) (Accel%20Change :type Boolean))
  (Physics|AddForce Target (* Strength (Math|Vector|Normalize (- Destination (Transformation|GetWorldLocation Target)))) "None" Accel%20Change))