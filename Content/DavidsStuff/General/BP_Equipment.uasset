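; Equipment Blueprint that tracks the selected slot among ten and handles switching and stowing.
; The swap axis cycles slots with wraparound through a gate that ADS closes for one equipment type and reopens on release.
; Wield/stow toggles between the remembered slot and none.
; Changes call EquipmentChanged, whose owner camera FOV and transform update is disabled, as are the direct slot-key selections.
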(event Custom|Equipment%20Changed
  (bind _asspeelbnio (Utilities|Casting|CastTo (Components|GetOwner)))
  (Camera|SetFieldOfView (Variables|Default|GetFollowCamera _asspeelbnio) (.FOV (Utilities|Struct|BreakEquipmentStruct (Utilities|Array|Get(acopy) (Variables|Default|GetEquipmentSlots) (Variables|Default|GetSelectedSlot)))))
  (Transformation|SetRelativeTransform (Variables|Default|GetFollowCamera _asspeelbnio) (.Camera (Utilities|Struct|BreakEquipmentStruct (Utilities|Array|Get(acopy) (Variables|Default|GetEquipmentSlots) (Variables|Default|GetSelectedSlot)))) false false)
  (if (Utilities|Enum|Equal(Enum) (.EquipmentType (Utilities|Struct|BreakEquipmentStruct (Utilities|Array|Get(acopy) (Variables|Default|GetEquipmentSlots) (Variables|Default|GetSelectedSlot)))) "NewEnumerator2")
    _))

(event EventBeginPlay
  (CallFunction|EquipmentChanged))

(event EventTick
  (params (DeltaSeconds :type Float%20%28single-precision%29)))

(event Input|ActionEvents|InputActionWeild/Stow
  (params (Key :type Key%20Structure :default "None"))
  (:Pressed
    (if (== (Variables|Default|GetStowedSlot) -1)
      (Variables|Default|SetStowedSlot (Variables|Default|GetSelectedSlot))
      (Variables|Default|SetSelectedSlot -1)
      (else
        (Variables|Default|SetSelectedSlot (Variables|Default|GetStowedSlot))
        (Variables|Default|SetStowedSlot -1)))
    (CallFunction|EquipmentChanged)))

(event Input|ActionEvents|InputActionADS
  (params (Key :type Key%20Structure :default "None"))
  (:Pressed
    (if (Utilities|Enum|Equal(Enum) (.EquipmentType (Utilities|Struct|BreakEquipmentStruct (Utilities|Array|Get(acopy) (Variables|Default|GetEquipmentSlots) (Variables|Default|GetSelectedSlot)))) "NewEnumerator1")
      (Utilities|FlowControl|Gate true) ; enters at Close
    ))
  (:Released
    (Utilities|FlowControl|Gate true) ; enters at Open
  ))

(event Input|ActionEvents|InputActionEquipment7
  (params (Key :type Key%20Structure :default "None"))
  (:Pressed
    (Variables|Default|SetSelectedSlot 7)
    (CallFunction|EquipmentChanged)))

(event Input|ActionEvents|InputActionEquipment6
  (params (Key :type Key%20Structure :default "None"))
  (:Pressed
    (Variables|Default|SetSelectedSlot 6)
    (CallFunction|EquipmentChanged)))

(event Input|ActionEvents|InputActionEquipment1
  (params (Key :type Key%20Structure :default "None"))
  (:Pressed
    (Variables|Default|SetSelectedSlot 1)
    (CallFunction|EquipmentChanged)))

(event Input|ActionEvents|InputActionEquipment2
  (params (Key :type Key%20Structure :default "None"))
  (:Pressed
    (Variables|Default|SetSelectedSlot 2)
    (CallFunction|EquipmentChanged)))

(event Input|ActionEvents|InputActionEquipment3
  (params (Key :type Key%20Structure :default "None"))
  (:Pressed
    (Variables|Default|SetSelectedSlot 3)
    (CallFunction|EquipmentChanged)))

(event Input|ActionEvents|InputActionEquipment4
  (params (Key :type Key%20Structure :default "None"))
  (:Pressed
    (Variables|Default|SetSelectedSlot 4)
    (CallFunction|EquipmentChanged)))

(event Input|ActionEvents|InputActionEquipment5
  (params (Key :type Key%20Structure :default "None"))
  (:Pressed
    (Variables|Default|SetSelectedSlot 5)
    (CallFunction|EquipmentChanged)))

(event Input|ActionEvents|InputActionEquipment10
  (params (Key :type Key%20Structure :default "None"))
  (:Pressed
    (Variables|Default|SetSelectedSlot 10)
    (CallFunction|EquipmentChanged)))

(event Input|ActionEvents|InputActionEquipment9
  (params (Key :type Key%20Structure :default "None"))
  (:Pressed
    (Variables|Default|SetSelectedSlot 9)
    (CallFunction|EquipmentChanged)))

(event Input|ActionEvents|InputActionEquipment8
  (params (Key :type Key%20Structure :default "None"))
  (:Pressed
    (Variables|Default|SetSelectedSlot 8)
    (CallFunction|EquipmentChanged)))

(event Input|AxisEvents|InputAxisSwapActive
  (params (AxisValue :type Float%20%28single-precision%29))
  (Utilities|FlowControl|Gate true
    (:Exit
      (Variables|Default|SetSelectedSlot (+ (Math|Integer|%(Integer) (+ (Math|Integer|%(Integer) (+ (Math|Float|Round AxisValue) (Variables|Default|GetSelectedSlot) -1) 10) 10) 10) 1))
      (CallFunction|EquipmentChanged))))