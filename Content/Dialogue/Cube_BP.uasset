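; Quest target cube that attaches itself to the player on contact and completes the quest referencing it.
; A hit from BP_ThirdPersonCharacter sets its IsOverlapped flag, disables cube collision and starts a next-tick loop that teleports the cube to the character's location.
; The loop's completion path searches ActiveQuests for this actor, calls QuestComplete on the character and fires EventQuestComplete on NPCs with a matching quest name.
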(event OnComponentHit(Cube)
  (params (HitComponent :type Primitive%20Component%20Object%20Reference) (OtherActor :type Actor%20Object%20Reference) (OtherComp :type Primitive%20Component%20Object%20Reference) (NormalImpulse :type Vector :default "0, 0, 0") (Hit :type Hit%20Result%20Structure%20%28by%20ref%29))
  (bind _asbp_third_person_character (Utilities|Casting|CastToBP_ThirdPersonCharacter OtherActor))
  (bind _output_get (Variables|/Game/ThirdPerson/Blueprints/BP_ThirdPersonCharacter.BP_ThirdPersonCharacter_C|SetisOverlapped? _asbp_third_person_character true))
  (if _output_get
    (for _index (range 0 0) :!label _label
      (Transformation|SetActorLocation (Transformation|GetActorLocation OtherActor) false false)
      (Collision|SetCollisionEnabled (Variables|Default|GetCube) "NoCollision")
      (Rendering|SetVisibility (Variables|Default|GetCube) true false)
      (Utilities|FlowControl|DelayUntilNextTick)
      (goto _label))
    (for _array_element (Variables|/Game/ThirdPerson/Blueprints/BP_ThirdPersonCharacter.BP_ThirdPersonCharacter_C|GetActiveQuests _asbp_third_person_character)
      (if (== self (.actorreference (Variables|/Game/Dialogue/BP_Quest.BP_Quest_C|GetQuestInfo _array_element)))
        (Default|QuestComplete _asbp_third_person_character _array_element)
        (bind _outactors (Actor|GetAllActorsOfClass "/Game/Dialogue/NPC.NPC_C"))
        (for _array_element_2 _outactors
          (if (Utilities|Enum|Equal(Enum) (.questname (Variables|/Game/Dialogue/BP_Quest.BP_Quest_C|GetQuestInfo _array_element)) (.questname (Variables|/Game/Dialogue/NPC.NPC_C|GetQuestRef _array_element_2)))
            (Default|EventQuestComplete _array_element_2)))))))

(fn ConstructionScript)